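; BP_PC is a player controller that toggles the pause menu.
; It creates the WBP_PauseMenu widget once on BeginPlay and reuses it for each pause.
; The Pause input either pauses the game, shows the menu and cursor and switches to UI-only input, or runs the reverse path.
; A separate UnPause event exposes that same resume path.
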(event Custom|UnPause
  (Game|SetGamePaused false)
  (Widget|RemovefromParent (Variables|Default|GetPauseMenu))
  (Variables|Default|SetbShowMouseCursor false)
  (Input|SetInputModeGameOnly self))

(event EventBeginPlay
  (bind _returnvalue (UserInterface|CreateWidget "/Game/Widgets/WBP_PauseMenu.WBP_PauseMenu_C"))
  (Variables|Default|SetPauseMenu _returnvalue))

(event Input|ActionEvents|InputActionPause
  (params (Key :type Key%20Structure :default "None"))
  (bind _self self)
  (bind _pausemenu (Variables|Default|GetPauseMenu))
  (:Pressed
    (if (Game|IsGamePaused)
      (Game|SetGamePaused false)
      (Widget|RemovefromParent _pausemenu)
      (Variables|Default|SetbShowMouseCursor false)
      (Input|SetInputModeGameOnly _self)
      (else
        (Game|SetGamePaused true)
        (UserInterface|Viewport|AddtoViewport _pausemenu 0)
        (Variables|Default|SetbShowMouseCursor true)
        (Input|SetInputModeUIOnly _self 0 "DoNotLock")))))

(fn ConstructionScript)