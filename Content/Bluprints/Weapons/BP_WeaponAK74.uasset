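; AK74 weapon Blueprint with automatic hitscan fire as the main attack and a grenade launcher as the alt attack.
; Main attack fires at once, then repeats on a looping ShotRate timer, spending ammo and playing effects until stopped or empty.
; Alt attack spawns a projectile at DirAlt with its own effects and no ammo check here.
; The attack overrides replace the parent logic without calling it.
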(event Custom|MakeOneShot
  ;[1 1 1] MakeOneShot
  (bind _result (CallFunction|SpendAmmo true))
  (if _result
    (CallFunction|MakeTraceShot true)
    (Components|Activation|Activate (Variables|Default|GetMain_ShotSound) true)
    (else
      (CallFunction|StopBurst))))

(event Custom|StartBurst
  ;[1 1 1] StartBurst
  (CallFunction|MakeOneShot)
  (bind _returnvalue (Utilities|Time|SetTimerbyEvent (delegate Custom|MakeOneShot) (Variables|Default|GetShotRate) true))
  (Variables|Default|SetBurstTM _returnvalue))

(event Custom|StopBurst
  ;[1 1 1] StopBurst
  (Utilities|Time|ClearandInvalidateTimerbyHandle (Variables|Default|GetBurstTM)))

(event Custom|LaunchGrenade
  ;[1 1 1] LaunchGrenade
  (Game|SpawnActorfromClass (Variables|Default|GetProjectileClass) (Transformation|GetWorldTransform (Variables|Default|GetDir_Alt)) "Undefined" 0 0)
  (Components|Activation|Activate (Variables|Default|GetAlt_ShotSound) true))

(fn ConstructionScript
  (|CallParentFunction))

(fn TryMainAttack
  (CallFunction|StartBurst))

(fn StopMainAttack
  (CallFunction|StopBurst))

(fn TryAltAttack
  (CallFunction|LaunchGrenade))