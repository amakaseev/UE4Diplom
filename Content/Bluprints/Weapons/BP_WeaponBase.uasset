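; Base weapon Blueprint providing main and alt fire functions, with the attack functions left as stubs that only print or do nothing.
; MakeTraceShot sphere-traces from the player camera along a random scatter cone, using per-mode spread and range, but applies no damage.
; It draws a debug line from the mode's direction component to the impact or trace end.
; SpendAmmo decrements the chosen ammo pool and reports success.
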(event EventBeginPlay)

(event Collision|EventActorBeginOverlap
  (params (OtherActor :type Actor%20Object%20Reference)))

(event EventTick
  (params (DeltaSeconds :type Float%20%28single-precision%29)))

(fn ConstructionScript)

(fn TryMainAttack
  (Development|PrintString "MAIN"))

(fn TryAltAttack
  (Development|PrintString "ALT"))

(fn MakeTraceShot
  (params (Main? :type Boolean))
  (bind _returnvalue (Game|GetPlayerCameraManager 0))
  (bind _returnvalue_2 (Camera|GetCameraLocation _returnvalue))
  (bind _outhit (Collision|SphereTraceByChannel _returnvalue_2 (+ _returnvalue_2 (* (Math|Random|RandomUnitVectorinConeinDegrees (Transformation|GetActorForwardVector _returnvalue) (select Main? (Variables|Damage|GetMainScatter) (Variables|Damage|GetAltScatter))) (select Main? (Variables|Damage|GetMainShotDistance) (Variables|Damage|GetAltShotDistance)))) 5.0 "TraceTypeQuery1" true 0 "None"))
  (Rendering|Debug|DrawDebugLine :LineStart (Transformation|GetWorldLocation (select Main? (Variables|Default|GetDir_Main) (Variables|Default|GetDir_Alt))) :LineEnd (select (.bBlockingHit (Collision|BreakHitResult _outhit)) (.ImpactPoint (Collision|BreakHitResult _outhit)) (.TraceEnd (Collision|BreakHitResult _outhit))) :Duration 2.0))

(fn StopMainAttack)

(fn SpendAmmo
  (params (Main? :type Boolean))
  (if (> (select Main? (Variables|Ammo|GetCurrentAmmo) (Variables|Ammo|GetCurrentAltAmmo)) 0)
    (Math|Integer|DecrementInt (select Main? (Variables|Ammo|GetCurrentAmmo) (Variables|Ammo|GetCurrentAltAmmo))
      (:%20%20
        (return true)))
    (else
      (return false))))