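; BP_WeaponM16 is the M16 weapon Blueprint, overriding the main and alt attack functions of its parent weapon class without calling the parent versions.
; Main attack spends ammo and, on success, makes a trace shot and activates the main shot sound and muzzle particle.
; Alt attack only makes a trace shot flagged as non-main, with no ammo check or effects in this Blueprint.
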(event EventBeginPlay
  (|CallParentFunction) ; This node is disabled and will not be called.\nDrag off pins to build functionality.
)

(event Collision|EventActorBeginOverlap
  (params (OtherActor :type Actor%20Object%20Reference))
  (|CallParentFunction OtherActor) ; This node is disabled and will not be called.\nDrag off pins to build functionality.
)

(event EventTick
  (params (DeltaSeconds :type Float%20%28single-precision%29))
  (|CallParentFunction DeltaSeconds) ; This node is disabled and will not be called.\nDrag off pins to build functionality.
)

(fn ConstructionScript
  (|CallParentFunction))

(fn TryMainAttack
  (bind _result (CallFunction|SpendAmmo true))
  (if _result
    (CallFunction|MakeTraceShot true)
    (Components|Activation|Activate (Variables|Default|GetMain_ShotSound) true)))

(fn TryAltAttack
  (CallFunction|MakeTraceShot false))