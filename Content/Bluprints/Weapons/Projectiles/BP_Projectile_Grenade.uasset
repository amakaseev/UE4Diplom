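; Grenade projectile Blueprint that explodes two seconds after spawning or immediately on hitting an actor tagged Enemy.
; Both the timer and the Sphere hit route into an Explode event, guarded by a DoOnce so it fires only once.
; Explode spawns a particle effect, sound and temporary scorch decal at its location, then destroys the actor; no damage is applied in this graph.
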(event OnComponentHit(Sphere)
  (params (HitComponent :type Primitive%20Component%20Object%20Reference) (OtherActor :type Actor%20Object%20Reference) (OtherComp :type Primitive%20Component%20Object%20Reference) (NormalImpulse :type Vector :default "0, 0, 0") (Hit :type Hit%20Result%20Structure%20%28by%20ref%29))
  (if (Actor|ActorHasTag OtherActor "Enemy")
    (CallFunction|Explode)))

(event Custom|Explode
  (bind _returnvalue (Transformation|GetActorLocation))
  (Utilities|FlowControl|DoOnce false
    (:Completed
      (Utilities|FlowControl|Sequence
        (:then_0
          (Effects|SpawnEmitteratLocation "/Game/AssetsStore/MilitaryWeapDark/FX/P_Grenade_Explosion_01.P_Grenade_Explosion_01" _returnvalue)
          (Audio|SpawnSoundatLocation "/Game/AssetsStore/MilitaryWeapDark/Sound/GrenadeLauncher/GrenadeLauncher_Explosion_Cue.GrenadeLauncher_Explosion_Cue" _returnvalue "0, 0, 0" 1.0 1.0 0.0 0 0)
          (Rendering|Decal|SpawnDecalatLocation "/Game/AssetsStore/BallisticsVFX/Decals/Decals_Scorch.Decals_Scorch" "20.000000,56.000000,56.000000" _returnvalue (Transformation|GetActorRotation) 1e+01))
        (:then_1
          (Actor|DestroyActor))))))

(event EventBeginPlay
  (|CallParentFunction)
  (Utilities|FlowControl|Delay 2.0)
  (CallFunction|Explode))

(fn ConstructionScript)